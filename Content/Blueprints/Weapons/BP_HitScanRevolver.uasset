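; Hitscan revolver weapon Blueprint that supplies procedural fire and reload animations for its static mesh.
; FireAnimation replays a Recoil timeline that drives the mesh's relative roll, while ReloadAnimation replays a Reload timeline that drives its relative Z position.
; The reload timeline holds IsReloading true while it plays and clears it on finish.
; No trace, damage or ammo logic is in these graphs.
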(event `self.FireAnimation`
  (bind _staticmesh (`self.StaticMesh`))
  (bind (_relativerotation_roll _relativerotation_pitch _relativerotation_yaw) (`KismetMathLibrary.BreakRotator` (`SceneComponent.RelativeRotation` _staticmesh)))
  (bind (_direction _recoil) (`Timeline|Recoil` :!via `PlayFromStart`)
    (:`Update`
      (`SceneComponent.K2_SetRelativeRotation` _staticmesh (`KismetMathLibrary.MakeRotator` _recoil _relativerotation_pitch _relativerotation_yaw) false false))))

(event `self.ReloadAnimation`
  (bind _staticmesh (`self.StaticMesh`))
  (bind (_relativelocation_x _relativelocation_y) (`KismetMathLibrary.BreakVector` (`SceneComponent.RelativeLocation` _staticmesh)))
  (bind (_direction _reload) (`Timeline|Reload` :!via `PlayFromStart`)
    (:`Update`
      (set `self.IsReloading` true)
      (`SceneComponent.K2_SetRelativeLocation` _staticmesh (`KismetMathLibrary.MakeVector` _relativelocation_x _relativelocation_y _reload) false false))
    (:`Finished`
      (set `self.IsReloading` false))))

(fn `UserConstructionScript`)