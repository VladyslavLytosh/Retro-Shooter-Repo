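; BP_MainCharacter is the main character Blueprint, which sets up the player HUD and drives movement-based camera shake.
; BeginPlay creates the WB_Hud widget and adds it to the viewport.
; Every Tick, CameraShakeHandler starts BP_FastShake on player controller 0 when the character moves above a speed threshold without falling, and BP_SlowShake otherwise.
; The shake start is re-issued each frame rather than only on state changes.
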(event `self.ReceiveTick`
  (params (DeltaSeconds :type "Float (single-precision)"))
  (`self.CameraShakeHandler`))

(event `self.ReceiveBeginPlay`
  (bind _returnvalue (`|CreateWidget` "/Game/UI/WB_Hud.WB_Hud_C"))
  (`UserWidget.AddToViewport` _returnvalue 0))

(fn `CameraShakeHandler`
  (bind _returnvalue (`GameplayStatics.GetPlayerController` 0))
  ;[1 0.2876 0.2378] Camera Shake Handler. Start camera shakes from different condition
  (if (and (> (`KismetMathLibrary.VSize` (`self.GetVelocity`)) 300.0) (not (`NavMovementComponent.IsFalling` (`self.CharacterMovement`))))
    (`PlayerController.ClientStartCameraShake` :`self` _returnvalue :`Shake` "/Game/Blueprints/CameraShake/BP_FastShake.BP_FastShake_C")
    (else
      (`PlayerController.ClientStartCameraShake` :`self` _returnvalue :`Shake` "/Game/Blueprints/CameraShake/BP_SlowShake.BP_SlowShake_C"))))

(fn `UserConstructionScript`)